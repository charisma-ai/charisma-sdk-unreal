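; BP_CharismaGameModeTemplate is a template game mode that starts a Charisma story conversation when play begins.
; On BeginPlay it requests a playthrough token for a hardcoded story and API key, stores the playthrough on the game mode, then creates a conversation.
; It attaches handlers and connects, starts the playthrough with speech enabled once ready, and prints each incoming message's text.
; Only success paths are handled.
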(event `self.ReceiveBeginPlay`
  (bind (_playthrough _token _playthroughuuid) (`CreatePlaythroughToken.CreatePlaythroughToken` 1863 -1 "4a0f0e29-152a-4ba5-af81-45538a4c5a31")
    (:`Success`
      (bind _output_get (set `self.Playthrough` _playthrough))
      (set `CharismaGameModeComponent.Playthrough` _output_get (`self.CharismaGameMode`))
      (set `self.PlaythroughUuid` _playthroughuuid)
      (bind _output_get_2 (set `self.PlaythroughToken` _token))
      (bind _conversationuuid (`CreateConversation.CreateConversation` _output_get_2)
        (:`Success`
          (bind _output_get_3 (set `self.ConversationUuid` _conversationuuid))
          (bind (_conversationid _isconnected _istyping _messageevent) (`PlaythroughEventsManager.AttachPlaythroughHandlers` _output_get)
            (:`then`
              (`Playthrough.Connect` _output_get))
            (:`OnReady`
              (`Playthrough.Start` _output_get _output_get_3 0 0 "" true))
            (:`OnMessage`
              (`KismetSystemLibrary.PrintString` (`.Text` (break `CharismaMessage` (`.Message` (break `CharismaMessageEvent` _messageevent))))))))))))

(fn `UserConstructionScript`)